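; Player character for parkour movement, with mouse look, strafe camera tilt, sliding and wall jumping.
; Holding LeftShift slides by shrinking the capsule and cutting ground friction.
; While falling, Tick traces to both sides, and Space launches the character up and away from a detected wall, otherwise jumping when grounded.
; Tick also drives speed-based FOV and the opacity of a speedlines widget through a dynamic material created on BeginPlay.
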(event EventTick
  (params (DeltaSeconds :type Float%20%28single-precision%29))
  (bind _camera (Variables|Default|GetCamera))
  (bind _capsulecomponent (Variables|Collision|GetCapsuleComponent))
  (bind _returnvalue (Transformation|GetWorldLocation _capsulecomponent))
  (bind _returnvalue_2 (Math|Vector|GetRightVector _capsulecomponent))
  (Variables|Default|Set%28DO%20NOT%20CHANGE%29%20Delta%20Seconds DeltaSeconds)
  (Utilities|FlowControl|Sequence
    (:then_0
      ;[1 0 0.0312] WallJump
      (if (AI|Components|NavMovement|IsFalling (Variables|Character|GetCharacterMovement))
        (bind _returnvalue_3 (Collision|LineTraceByChannel _returnvalue (+ _returnvalue (* _returnvalue_2 4e+01)) "TraceTypeQuery1" false 0 "None"))
        (bind _returnvalue_4 (Collision|LineTraceByChannel _returnvalue (+ _returnvalue (* _returnvalue_2 -4e+01)) "TraceTypeQuery1" false 0 "None" true "(R=0.000000,G=1.000000,B=0.081864,A=1.000000)" "(R=1.000000,G=0.014920,B=0.000000,A=1.000000)"))))
    (:then_1
      ;[0 1 0.8515] Speed Lines Opacity
      (Rendering|Material|SetScalarParameterValue (Variables|Default|Get%28DO%20NOT%20CHANGE%29Speedline%20Material%20Instance) "Opacity" (Math|Float|NormalizetoRange (Math|Vector|VectorLength (Variables|/Script/Engine.MovementComponent|GetVelocity (Variables|Character|GetCharacterMovement))) 0.0 1.2e+04) :!class /Script/Engine.MaterialInstanceDynamic))
    (:then_2
      ;[0 0.5625 0.05144] FOV Effects
      (if (>= (Math|Vector|VectorLength (Variables|/Script/Engine.MovementComponent|GetVelocity (Variables|Character|GetCharacterMovement))) (Variables|Default|GetFOV%20Change%20Speed))
        (Camera|SetFieldOfView _camera (Math|Interpolation|FInterpTo (Variables|/Script/Engine.CameraComponent|GetFieldOfView _camera) (+ (Variables|Default|GetFOV%20Original) (Variables|Default|GetFOV%20Increase%20Increment)) (Variables|Default|Get%28DO%20NOT%20CHANGE%29%20Delta%20Seconds) (Variables|Default|GetFOV%20Increase%20Speed)))
        (else
          (Camera|SetFieldOfView _camera (Math|Interpolation|FInterpTo (Variables|/Script/Engine.CameraComponent|GetFieldOfView _camera) (Variables|Default|GetFOV%20Original) (Variables|Default|Get%28DO%20NOT%20CHANGE%29%20Delta%20Seconds) (Variables|Default|GetFOV%20Decrease%20Speed))))))))

(event EventBeginPlay
  (Utilities|FlowControl|Sequence
    (:then_0
      ;[1 0.9245 0] Create Speedlines widget
      (bind _returnvalue (UserInterface|CreateWidget "/Game/ParkourMovementPack/Widgets/WBP_Speedlines.WBP_Speedlines_C"))
      (bind _output_get (Variables|Default|Set%28DO%20NOT%20CHANGE%29Speedline%20widget _returnvalue))
      (UserInterface|Viewport|AddtoViewport _output_get 0)
      (bind _returnvalue_2 (Rendering|Material|CreateDynamicMaterialInstance (Class|WidgetBlueprintLibrary|GetBrushResourceasMaterial (Variables|/Script/UMG.Image|GetBrush (Variables|/Game/ParkourMovementPack/Widgets/WBP_Speedlines.WBP_Speedlines_C|GetSpeedlineImage (Variables|Default|Get%28DO%20NOT%20CHANGE%29Speedline%20widget)))) "None" "None" :!class /Script/Engine.KismetMaterialLibrary))
      (bind _output_get_2 (Variables|Default|Set%28DO%20NOT%20CHANGE%29Speedline%20Material%20Instance _returnvalue_2))
      (Class|WidgetBlueprintLibrary|SetBrushResourcetoMaterial (Variables|/Script/UMG.Image|GetBrush (Variables|/Game/ParkourMovementPack/Widgets/WBP_Speedlines.WBP_Speedlines_C|GetSpeedlineImage (Variables|Default|Get%28DO%20NOT%20CHANGE%29Speedline%20widget))) _output_get_2))
    (:then_1
      (Variables|Default|SetFOV%20Original (Variables|/Script/Engine.CameraComponent|GetFieldOfView (Variables|Default|GetCamera))))))

(event Input|AxisEvents|InputAxisRight/left
  (params (AxisValue :type Float%20%28single-precision%29))
  (bind _returnvalue (Pawn|GetControlRotation :!class /Script/Engine.Pawn))
  ;[1 1 1] Movement Logic
  (Pawn|Input|AddMovementInput (Math|Vector|GetRightVector (Variables|Collision|GetCapsuleComponent)) AxisValue false)
  ;[0 1 0.8988] Camera Tilt
  (Variables|Default|SetCamera%20Tilt%20Current (Math|Interpolation|FInterpTo (Variables|Default|GetCamera%20Tilt%20Current) (* AxisValue (Variables|Default|GetCamera%20Tilt%20Amount)) (Variables|Default|Get%28DO%20NOT%20CHANGE%29%20Delta%20Seconds) (Variables|Default|GetCamera%20Tilt%20Speed)))
  (Transformation|SetRelativeRotation (Variables|Default|GetCamera) (Math|Rotator|MakeRotator (Math|Interpolation|FInterpTo (Variables|Default|GetCamera%20Tilt%20Current) (* AxisValue (Variables|Default|GetCamera%20Tilt%20Amount)) (Variables|Default|Get%28DO%20NOT%20CHANGE%29%20Delta%20Seconds) (Variables|Default|GetCamera%20Tilt%20Speed)) (.pitch _returnvalue) (.yaw _returnvalue)) false false))

(event Input|AxisEvents|InputAxisMouseUp/Down
  (params (AxisValue :type Float%20%28single-precision%29))
  ;[1 1 1] Camera Logic
  (Pawn|Input|AddControllerPitchInput AxisValue))

(event Input|AxisEvents|InputAxisMouseRight/Left
  (params (AxisValue :type Float%20%28single-precision%29))
  ;[1 1 1] Camera Logic
  (Pawn|Input|AddControllerYawInput AxisValue))

(event Input|AxisEvents|InputAxisForwards/Backwards
  (params (AxisValue :type Float%20%28single-precision%29))
  ;[1 1 1] Movement Logic
  (Pawn|Input|AddMovementInput (Math|Vector|GetForwardVector (Variables|Collision|GetCapsuleComponent)) AxisValue false))

(event Input|KeyboardEvents|SpaceBar
  (params (Key :type Key%20Structure :default "None"))
  (bind _walljump_force_up (Variables|Default|GetWallJump%20Force%20Up))
  (bind _capsulecomponent (Variables|Collision|GetCapsuleComponent))
  (bind _walljump_force_side (Variables|Default|GetWallJump%20Force%20Side))
  (bind _returnvalue (Math|Vector|GetRightVector _capsulecomponent))
  (bind _returnvalue_2 (Math|Vector|GetUpVector _capsulecomponent))
  (bind _returnvalue_3 (* _returnvalue_2 _walljump_force_up))
  ;[1 0 0.0312] WallJump
  (:Pressed
    (if (AI|Components|NavMovement|IsFalling (Variables|Character|GetCharacterMovement))
      (if (stale EventTick _returnvalue_3)
        (Character|LaunchCharacter (+ _returnvalue_3 (* _returnvalue (* _walljump_force_side -1.0))) false true)
        (Pawn|Input|AddControllerRollInput 0.0)
        (elif (stale EventTick _returnvalue_4)
          (Character|LaunchCharacter (+ _returnvalue_3 (* _returnvalue _walljump_force_side)) false true)))
      (else
        (Character|Jump)))))

(event Input|KeyboardEvents|LeftShift
  (params (Key :type Key%20Structure :default "None"))
  (bind _capsulecomponent (Variables|Collision|GetCapsuleComponent))
  (bind _charactermovement (Variables|Character|GetCharacterMovement))
  (bind _returnvalue (Components|Capsule|GetScaledCapsuleHalfHeight _capsulecomponent))
  ;[1 0.8678 0] Sliding Logic
  (:Pressed
    (Components|Capsule|SetCapsuleHalfHeight _capsulecomponent (/ _returnvalue 3.0) true)
    (Variables|/Script/Engine.CharacterMovementComponent|SetGroundFriction _charactermovement (/ (Variables|/Script/Engine.CharacterMovementComponent|GetGroundFriction _charactermovement) 1e+02)))
  (:Released
    (Components|Capsule|SetCapsuleHalfHeight _capsulecomponent (* _returnvalue 3.0) true)
    (Variables|/Script/Engine.CharacterMovementComponent|SetGroundFriction _charactermovement (* (Variables|/Script/Engine.CharacterMovementComponent|GetGroundFriction _charactermovement) 1e+02))))

(fn ConstructionScript)